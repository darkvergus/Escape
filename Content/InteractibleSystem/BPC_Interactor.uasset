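; Interactor component for the first-person character that handles interacting with world objects and holding one item in hand.
; Each Tick, a short camera line trace finds a BPI_Interactable that allows interaction, caching it as ActiveInteractible and toggling its prompt on the HUD widget.
; Interact messages that target; pick-ups replace any held item, which is dropped first.
; The held item can be dropped, thrown or consumed, with ItemMesh mirroring its mesh.
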(event `self.ReceiveBeginPlay`)

(event `self.ReceiveTick`
  (params (DeltaSeconds :type "Float (single-precision)"))
  (`self.RenderInteractionWidget`))

(fn `changeItemInHand`
  (bind _iteminhandobj (`self.itemInHandObj`))
  (bind _itemmesh (`self.itemMesh`))
  (`/Engine/EditorBlueprintResources/StandardMacros.IsValid` _iteminhandobj
    (:`Is Valid`
      (bind _asbase_pick_up (cast `/Game/InteractibleSystem/Base_PickUp` _iteminhandobj))
      (bind _itemmesh_2 (`/Game/InteractibleSystem/BPI_PickUpable.getItemMesh` _asbase_pick_up))
      (`StaticMeshComponent.SetStaticMesh` _itemmesh _itemmesh_2))
    (:`Is Not Valid`
      (`StaticMeshComponent.SetStaticMesh` _itemmesh null))))

(fn `ConsumeItem`
  (bind _iteminhandobj (`self.itemInHandObj`))
  (if (`KismetSystemLibrary.IsValid` _iteminhandobj)
    (bind _type (message `/Game/InteractibleSystem/BPI_PickUpable.getType` _iteminhandobj))
    (if (`|EnumEquality` _type "NewEnumerator2")
      (bind _asbase_consumable (cast `/Game/InteractibleSystem/Base_Consumable` _iteminhandobj))
      (`/Game/InteractibleSystem/Base_Consumable.Consume` _asbase_consumable)
      (`self.destroyItemInHand`))))

(fn `destroyItemInHand`
  (`Actor.K2_DestroyActor` (`self.itemInHandObj`))
  (set `self.itemInHandObj` null)
  (`self.changeItemInHand`))

(fn `dropItem`
  (bind _returnvalue (`self.GetOwner`))
  (message `/Game/InteractibleSystem/BPI_PickUpable.Drop` (`self.itemInHandObj`) (+ (`SceneComponent.K2_GetComponentLocation` (`Actor.RootComponent` _returnvalue)) (* (`Actor.GetActorForwardVector` _returnvalue) (`self.dropOffset`))))
  (set `self.itemInHandObj` null)
  (`self.changeItemInHand`))

(fn `GetActiveInteractible`
  (returns (AciveInteractible :type "Actor Object Reference"))
  (bind _asbp_first_person_character (cast `/Game/FirstPerson/Blueprints/BP_FirstPersonCharacter` (`self.GetOwner`))
    (:`then`
      (bind _firstpersoncamera (`/Game/FirstPerson/Blueprints/BP_FirstPersonCharacter.FirstPersonCamera` _asbp_first_person_character))
      (bind _returnvalue (`SceneComponent.GetSocketLocation` _firstpersoncamera "None"))
      (bind (_outhit _returnvalue_2) (`KismetSystemLibrary.LineTraceSingleForObjects` :`Start` _returnvalue :`End` (+ _returnvalue (* (`SceneComponent.GetForwardVector` _firstpersoncamera) 100.0)) :`ObjectTypes` (`|MakeArray` "ObjectTypeQuery2" :!type "EObjectTypeQuery Enum") :`DrawDebugType` "ForDuration" :`DrawTime` 0.1))
      (if _returnvalue_2
        (bind (_bblockinghit _binitialoverlap _time _distance _location _impactpoint _normal _impactnormal _physmat _hitactor) (`GameplayStatics.BreakHitResult` _outhit))
        (if (`KismetSystemLibrary.DoesImplementInterface` _hitactor "/Game/InteractibleSystem/BPI_Interactable.BPI_Interactable_C")
          (bind _caninteract (message `/Game/InteractibleSystem/BPI_Interactable.CanInteract` _hitactor))
          (if _caninteract
            (bind _output_get (set `self.ActiveInteractible` _hitactor))
            (return _output_get))
          (else
            (set `self.ActiveInteractible` null :!label _label)
            (return null)))
        (else
          (goto _label))))
    (:`CastFailed`
      (`KismetSystemLibrary.PrintText` "Interactor Error: Failed to cast to owner  " true true (struct :`R` 1.0 :`B` 0.017903 :`A` 1.0)))))

(fn `getItemInHand`
  (returns (itemInHandObj :type "Actor Object Reference"))
  (return (`self.itemInHandObj`)))

(fn `interact`
  (bind _returnvalue (`self.GetOwner`))
  (bind _activeinteractible (`self.ActiveInteractible`))
  (`/Engine/EditorBlueprintResources/StandardMacros.IsValid` _activeinteractible
    (:`Is Valid`
      (if (`KismetSystemLibrary.DoesImplementInterface` _activeinteractible "/Game/InteractibleSystem/BPI_PickUpable.BPI_PickUpable_C")
        (bind _isempty (`self.isLeftHandEmpty`))
        (if (not _isempty)
          (`self.dropItem`))
        (message `/Game/InteractibleSystem/BPI_Interactable.OnInteract` _activeinteractible _returnvalue)
        (set `self.itemInHandObj` _activeinteractible)
        (`self.changeItemInHand`)
        (else
          (message `/Game/InteractibleSystem/BPI_Interactable.OnInteract` _activeinteractible _returnvalue))))))

(fn `isLeftHandEmpty`
  (returns (isEmpty :type Boolean))
  (return (not (`KismetSystemLibrary.IsValid` (`self.itemInHandObj`)))))

(fn `RenderInteractionWidget`
  (bind _aciveinteractible (`self.GetActiveInteractible`))
  (bind _returnvalue (`PlayerController.GetHUD` (`GameplayStatics.GetPlayerController` 0)))
  (`/Engine/EditorBlueprintResources/StandardMacros.IsValid` _aciveinteractible
    (:`Is Valid`
      (bind _asnew_hud (cast `/Game/InteractibleSystem/NewHUD` _returnvalue))
      (bind _interactionprompt (message `/Game/InteractibleSystem/BPI_Interactable.GetInteractionPrompt` _aciveinteractible))
      (bind _ui_ref (`/Game/InteractibleSystem/NewHUD.UI_Ref` _asnew_hud))
      (`/Game/InteractibleSystem/Widget_Interaction.Change Interaction Text` _ui_ref (`KismetTextLibrary.Conv_TextToString` _interactionprompt))
      (`Widget.SetVisibility` _ui_ref "Visible"))
    (:`Is Not Valid`
      (bind _asnew_hud_2 (cast `/Game/InteractibleSystem/NewHUD` _returnvalue))
      (`Widget.SetVisibility` (`/Game/InteractibleSystem/NewHUD.UI_Ref` _asnew_hud_2) "Hidden"))))

(fn `throwItemInHand`
  (bind _iteminhandobj (`self.itemInHandObj`))
  (`/Engine/EditorBlueprintResources/StandardMacros.IsValid` _iteminhandobj
    (:`Is Valid`
      (bind _asbase_throwable (cast `/Game/InteractibleSystem/Base_Throwable` _iteminhandobj))
      (`/Game/InteractibleSystem/Base_Throwable.throwObj` _asbase_throwable (`Actor.GetActorForwardVector` (`self.GetOwner`)))
      (set `self.itemInHandObj` null)
      (`self.changeItemInHand`))))