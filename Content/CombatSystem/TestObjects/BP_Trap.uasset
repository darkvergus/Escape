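; BP_Trap is a test trap actor in the combat system that repeatedly raises and lowers its Scene component on a timed cycle.
; A self-repeating Attack event waits, then uses a FlipFlop to alternate the Sphere between query-only and no collision while passing the direction to MoveTrap.
; MoveTrap drives the vertical offset through a timeline played forward or reversed.
; The Sphere's overlap handler is empty, so contact has no effect.
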(event `self.ReceiveBeginPlay`
  (`PrimitiveComponent.SetCollisionEnabled` (`self.Sphere`) "NoCollision")
  (`self.Attack`))

(event `self.Sphere.OnComponentBeginOverlap`
  (params (OverlappedComponent :type "PrimitiveComponent Object Reference") (OtherActor :type "Actor Object Reference") (OtherComp :type "PrimitiveComponent Object Reference") (OtherBodyIndex :type Integer) (bFromSweep :type Boolean) (SweepResult :type "HitResult Structure (by ref)")))

(event `self.Attack`
  (`KismetSystemLibrary.Delay` 5.0)
  (`|ExecutionSequence`
    (:`then_0`
      (bind _isa (`/Engine/EditorBlueprintResources/StandardMacros.FlipFlop`)
        (:`A`
          (`PrimitiveComponent.SetCollisionEnabled` (`self.Sphere`) "QueryOnly"))
        (:`B`
          (`PrimitiveComponent.SetCollisionEnabled` (`self.Sphere`) "NoCollision")))
      (`self.MoveTrap` (0.0 0.0 50.0) 2.0 _isa)
      (`self.Attack`))))

(event `MoveTrap`
  (params (Movement :type "Vector Structure" :default (0.0 0.0 50.0)) (Duration :type "Float (double-precision)" :default 2.0) (FromBegin :type Boolean :default false))
  (if FromBegin
    (bind (_direction _alpha) (`Timeline|TrapMNoveTimeline` :`NewTime` Duration :!via `PlayFromStart` :!label _label)
      (:`Update`
        (`SceneComponent.K2_SetRelativeLocation` (`self.Scene`) (* Movement _alpha) false false)))
    (else
      (goto _label :!via `ReverseFromEnd`))))

(fn `UserConstructionScript`)