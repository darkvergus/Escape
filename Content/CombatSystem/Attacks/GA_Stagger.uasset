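; GA_Stagger is an event-triggered gameplay ability that knocks the avatar character back as a stagger.
; With a hit result in the event's target data, it launches the character away from the impact point by Strength, with a fixed upward lift.
; Without one, it adds only an unscaled forward-vector launch.
; Both branches end the ability after a Duration delay, and ending prints a debug string.
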(event `self.K2_ActivateAbilityFromEvent`
  (params (EventData :type "GameplayEventData Structure (by ref)"))
  (bind (_returnvalue_bblockinghit _returnvalue_binitialoverlap _returnvalue_time _returnvalue_distance _returnvalue_location _returnvalue_impactpoint) (`GameplayStatics.BreakHitResult` (`AbilitySystemBlueprintLibrary.GetHitResultFromTargetData` EventData_TargetData)))
  (`self.K2_CommitAbility`)
  (bind _ascharacter (cast `Character` (`self.GetAvatarActorFromActorInfo`)))
  (set `self.Target` _ascharacter)
  (if (`AbilitySystemBlueprintLibrary.TargetDataHasHitResult` EventData_TargetData)
    (bind _output_get (set `self.HitLocation` _returnvalue_impactpoint))
    (bind _output_get_2 (set `self.Dir` (`KismetMathLibrary.Normal` (- (`Actor.K2_GetActorLocation` (`self.GetAvatarActorFromActorInfo`)) _output_get))))
    (bind (_returnvalue_x _returnvalue_y) (`KismetMathLibrary.BreakVector` (* _output_get_2 (`self.strength`))))
    (`Character.LaunchCharacter` (`self.Target`) (`KismetMathLibrary.MakeVector` _returnvalue_x _returnvalue_y 100.0) true true)
    (`AbilityTask_WaitDelay.WaitDelay` (`self.Duration`)
      (:`OnFinish`
        (`self.K2_EndAbility`)))
    (else
      (`Character.LaunchCharacter` _ascharacter (`Actor.GetActorForwardVector` (`self.Target`)) false false)
      (`AbilityTask_WaitDelay.WaitDelay` (`self.Duration`)
        (:`OnFinish`
          (`self.K2_EndAbility`))))))

(event `self.K2_OnEndAbility`
  (params (bWasCancelled :type Boolean))
  (`KismetSystemLibrary.PrintString` "Back "))