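; Example damageable actor for the combat system that prints feedback when hit and respawns after death.
; ReceiveDamage forwards damage to a Breakable component and prints the damage and current health.
; On death it waits DestroyTimer, spawns a fresh copy at the root transform cached on BeginPlay, then destroys itself.
; The other damage functions are stubs: CanBeDamaged returns false, health getters return zero, and TryBlock never blocks.
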(event `self.ReceiveBeginPlay`
  (set `self.Init Transform` (`SceneComponent.K2_GetComponentToWorld` (`self.DefaultSceneRoot`))))

(event `self.Breakable.OnDeath`
  (`KismetSystemLibrary.PrintText` (`|FormatText` "{this} >  I Died " (`KismetSystemLibrary.GetObjectName` self)))
  (`KismetSystemLibrary.Delay` (`self.destroy timer`))
  (`|SpawnActorFromClass` (`GameplayStatics.GetObjectClass` self) (`self.Init Transform`) "Undefined" "MultiplyWithRoot" null null)
  (`self.K2_DestroyActor`))

(fn `CanBeDamaged`
  (returns (ReturnValue :type Boolean))
  (return false))

(fn `GetCurrentHealth`
  (returns (ReturnValue :type "Float (single-precision)"))
  (return 0.0))

(fn `GetMaxHealth`
  (returns (ReturnValue :type "Float (single-precision)"))
  (return 0.0))

(fn `ReceiveDamage`
  (params (DamageInfo :type "DamageInfo Structure (by ref)"))
  (returns (ReturnValue :type "EDamageResult Enum"))
  (bind _breakable (`self.Breakable`))
  (`KismetSystemLibrary.PrintText` (`|FormatText` "OUCH YOUR HURTING ME! {damage}  Damage" (`.Damage` (break `DamageInfo` DamageInfo))) true true (struct :`R` 1.0 :`G` 0.252461 :`A` 1.0))
  (bind _returnvalue (`IDamageableInterface.ReceiveDamage` _breakable DamageInfo))
  (`KismetSystemLibrary.PrintText` (`|FormatText` (`KismetTextLibrary.Conv_DoubleToText` (`BreakableComponent.CurrentHealth` _breakable) "HalfToEven")) true true (struct :`R` 0.227259 :`G` 1.0 :`A` 1.0))
  (return _returnvalue))

(fn `TryBlock`
  (params (DamageInfo :type " Structure (by ref)"))
  (returns (ReturnValue :type "EBlockResult Enum"))
  (return "NotBlocking"))

(fn `UserConstructionScript`)