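; BP_Attacker is an example enemy from the sword animation pack that endlessly swings its sword to hit the player.
; BeginPlay starts the Attacking event, which plays a right-top swing montage and calls itself again when the montage completes.
; On a montage notify, it checks whether its Box overlaps player character 0 and, if so, sends that character HitMessage.
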(event `self.ReceiveBeginPlay`
  (`self.Attacking`))

(event `Attacking`
  (bind _returnvalue (`GameplayStatics.GetPlayerCharacter` 0))
  (`|PlayMontage` (`self.SkeletalMesh`) "/Game/SwordAnimationPack/Characters/AttackerExample/Swing_RightTop_Full_Montage.Swing_RightTop_Full_Montage"
    (:`OnCompleted`
      (set `self.Busy` false)
      (`self.Attacking`))
    (:`OnNotifyBegin`
      (if (`PrimitiveComponent.IsOverlappingActor` (`self.Box`) _returnvalue)
        (message `/Game/SwordAnimationPack/Demo/Blueprints/BPI_SwordPlayer.Hit` _returnvalue)))))

(fn `UserConstructionScript`)